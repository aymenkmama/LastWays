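; Player controller for the main menu that prepares the menu inventory, pawn and input on BeginPlay.
; For the local controller only, it spawns and stores a Bp_MainMenuInventory actor, passing itself as that actor's MainMenuPawn.
; It then shows the cursor, disables the MainMenuPawn's movement, flips its mesh 180 degrees and switches to UI-only input focused on MainMenuMainWidget.
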(event `self.ReceiveBeginPlay`
  (if (`self.IsLocalPlayerController`)
    (set `self.MainMenuController` true)
    (bind _returnvalue (`|SpawnActorFromClass` "/Game/UI/MainMenu/BluePrintMainMenuInventory/Bp_MainMenuInventory.Bp_MainMenuInventory_C" (`KismetMathLibrary.MakeTransform` (0.0 0.0 0.0)) "AlwaysSpawn" "OverrideRootScale" null 20 self 4 null))
    (set `self.MMInventoryRef` _returnvalue)
    (set `PlayerController.bShowMouseCursor` true (`GameplayStatics.GetPlayerController` 0))
    (bind _asmain_menu_pawn (cast `/Game/BluePrints/Characters/CharacterBluePrints/MainMenuPawn` (`GameplayStatics.GetPlayerPawn` 0)))
    (`CharacterMovementComponent.DisableMovement` (`Character.CharacterMovement` _asmain_menu_pawn))
    (`SceneComponent.K2_AddLocalRotation` (`Character.Mesh` _asmain_menu_pawn) (struct :`Yaw` 180.0) false false)
    (`WidgetBlueprintLibrary.SetInputMode_UIOnlyEx` self (`self.MainMenuMainWidget`))))

(fn `UserConstructionScript`)