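; Battle-royale safe zone actor that shrinks a scaled wall in timed stages and damages living players caught outside it.
; The server registers it with GameState_Kma, then InitZone starts hold timers, each leading to a shrink toward a randomly offset center.
; Tick scales and moves the wall; each finished stage rescales hold and shrink times until radius drops below minimum.
; Server damage uses horizontal distance rather than overlaps, skipping players on the plane.
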(event `self.ReceiveBeginPlay`
  (`/Engine/EditorBlueprintResources/ActorMacros.Switch Has Authority`
    (:`Authority`
      (bind _asgame_state_kma (cast `/Game/BluePrints/AllLevels/GameState_Kma` (`GameplayStatics.GetGameState`)))
      (set `/Game/BluePrints/AllLevels/GameState_Kma.SafeZone` self _asgame_state_kma)
      (set `self.NextRadius` (* (`self.Radius`) (`self.ShrinkMultiplier`)))
      (set `self.ShrinkSpeed` (/ (- (`self.Radius`) (`self.NextRadius`)) (`self.ShrinkTime`)))
      (set `self.NextLocation` (`self.GetNextLocation`)))))

(event `BeginShrinking`
  (`/Engine/EditorBlueprintResources/ActorMacros.Switch Has Authority`
    (:`Authority`
      (`/Engine/EditorBlueprintResources/StandardMacros.IncrementInt` (`self.NumShrinks`)
        (:`  `
          (set `self.StartShrinkLocation` (`self.K2_GetActorLocation`))
          (set `self.Shrinking?` true)
          (set `self.BeginShrinkTime` (`GameplayStatics.GetTimeSeconds`))
          (set `self.ShrinkSpeed` (/ (- (`self.Radius`) (`self.NextRadius`)) (`self.ShrinkTime`)))
          (`self.SetActorHiddenInGame` false))))))

(event `InitZone`
  (`/Engine/EditorBlueprintResources/ActorMacros.Switch Has Authority`
    (:`Authority`
      (set `self.Enabled?` true)
      (`KismetSystemLibrary.K2_SetTimerDelegate` (delegate `BeginShrinking`) (`self.HoldTime`)))))

(event `self.ReceiveTick`
  (params (DeltaSeconds :type "Float (single-precision)"))
  (if (`self.Shrinking?`)
    (`self.UpDateWallTransform` DeltaSeconds))
  (if (`self.Enabled?`)
    (`/Engine/EditorBlueprintResources/ActorMacros.Switch Has Authority`
      (:`Authority`
        (`self.DamagePlayersOutsideWall` DeltaSeconds)))))

(event `UpDateWallTransform`
  (params (DeltaSeconds :type "Float (double-precision)"))
  (bind _radius (`self.Radius`))
  (set `self.Radius` (- (`self.Radius`) (* (`self.ShrinkSpeed`) DeltaSeconds)))
  (`self.SetActorScale3D` (`KismetMathLibrary.MakeVector` _radius _radius (`self.Height`)))
  (`self.K2_SetActorLocation` (`KismetMathLibrary.VInterpTo_Constant` (`self.K2_GetActorLocation`) (`self.NextLocation`) DeltaSeconds (/ (`KismetMathLibrary.VSize` (- (`self.StartShrinkLocation`) (`self.NextLocation`))) (`self.ShrinkTime`))))
  (if (and (`self.HasAuthority`) (>= (/ (- (`GameplayStatics.GetTimeSeconds`) (`self.BeginShrinkTime`)) (`self.ShrinkTime`)) 1.0))
    (set `self.Shrinking?` false)
    (set `self.HoldTime` (* (`self.HoldTime`) (`self.TimeMultiplier`)))
    (set `self.NextRadius` (* (`self.NextRadius`) (`self.ShrinkMultiplier`)))
    (set `self.NextLocation` (`self.GetNextLocation`))
    (set `self.ShrinkTime` (* (`self.ShrinkTime`) (`self.TimeMultiplier`)))
    (if (>= (`self.Radius`) (`self.MinRadius`))
      (`KismetSystemLibrary.K2_SetTimerDelegate` (delegate `BeginShrinking`) (`self.HoldTime`))
      (else
        (set `self.FinishShrinking` true)))))

(event `DamagePlayersOutsideWall`
  (params (DeltaSeconds :type "Float (double-precision)"))
  (bind _returnvalue (* (`self.WallDamagePerSecond`) DeltaSeconds))
  (bind _asgame_state_kma (cast `/Game/BluePrints/AllLevels/GameState_Kma` (`GameplayStatics.GetGameState`)))
  (if (and (`self.Enabled?`) (>= (`self.NumShrinks`) 0) (not (`self.bHidden`)) (`/Game/BluePrints/AllLevels/GameState_Kma.GameStarted?` _asgame_state_kma))
    (bind _asgame_mode_kma (cast `/Game/BluePrints/GamePlay/GameModeKma` (`GameplayStatics.GetGameMode`)))
    (for _array_element (`/Game/BluePrints/GamePlay/GameModeKma.ALivePlayersList` _asgame_mode_kma)
      (`/Engine/EditorBlueprintResources/StandardMacros.IsValid` _array_element
        (:`Is Valid`
          (if (not (`/Game/BluePrints/GamePlay/PlayerControllerKma.IsOnPlane?` _array_element))
            (bind _returnvalue_2 (`Controller.K2_GetPawn` _array_element))
            (if (>= (* (`self.GetHorizontalDistanceTo` self _returnvalue_2) 0.01) (* (`self.Radius`) 0.5))
              (`KismetSystemLibrary.PrintString` (`KismetStringLibrary.Conv_DoubleToString` _returnvalue))
              (`GameplayStatics.ApplyDamage` _returnvalue_2 _returnvalue null self "/Engine/EngineDamageTypes/DmgTypeBP_Environmental.DmgTypeBP_Environmental_C"))))))))

(fn `GetNextLocation`
  (returns (NextLocation :type "Vector Structure"))
  (bind _returnvalue (`self.K2_GetActorLocation`))
  (bind _z (.z _returnvalue))
  (bind _returnvalue_2 (* (- (`self.Radius`) (`self.NextRadius`)) 0.5))
  (bind _returnvalue_3 (* _returnvalue_2 -1.0))
  (return (`KismetMathLibrary.MakeVector` (.x (+ _returnvalue (`KismetMathLibrary.MakeVector` (* (`KismetMathLibrary.DegAcos` (`KismetMathLibrary.RandomFloatInRange` -180.0 180.0)) (`KismetMathLibrary.RandomFloatInRange` _returnvalue_3 _returnvalue_2)) (* (`KismetMathLibrary.DegAsin` (`KismetMathLibrary.RandomFloatInRange` -180.0 180.0)) (`KismetMathLibrary.RandomFloatInRange` _returnvalue_3 _returnvalue_2)) _z))) (.y (+ _returnvalue (`KismetMathLibrary.MakeVector` (* (`KismetMathLibrary.DegAcos` (`KismetMathLibrary.RandomFloatInRange` -180.0 180.0)) (`KismetMathLibrary.RandomFloatInRange` _returnvalue_3 _returnvalue_2)) (* (`KismetMathLibrary.DegAsin` (`KismetMathLibrary.RandomFloatInRange` -180.0 180.0)) (`KismetMathLibrary.RandomFloatInRange` _returnvalue_3 _returnvalue_2)) _z))) _z)))

(fn `UserConstructionScript`
  (bind _radius (`self.Radius`))
  (`SceneComponent.SetWorldScale3D` (`self.WallZoneSphere`) (`KismetMathLibrary.MakeVector` _radius _radius (`self.Height`))))