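; Player controller for a battle royale match, driving the local player's flow from lobby through plane drop to spectating and post-match.
; BeginPlay shows lobby UI; OnGameBegin spawns inventory, then force-drops anyone still aboard after the plane's timer.
; A camera line trace ends flight and spawns the parachute upon a hit.
; On death it possesses a spectator pawn attached to the killer, or shows the post-match screen without one.
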(event `ShowInGameHud`
  (if (`self.IsLocalController`)
    (bind _asbase_character_bp (cast `/Game/BluePrints/Characters/CharacterBluePrints/BaseCharacter_Bp` (`GameplayStatics.GetPlayerPawn` 0)))
    (set `PlayerController.bShowMouseCursor` true (`GameplayStatics.GetPlayerController` 0))
    (bind _returnvalue (`|SpawnActorFromClass` "/Game/InventorySystem/Bp_Inventory.Bp_Inventory_C" (`KismetMathLibrary.MakeTransform` (0.0 0.0 0.0)) "AlwaysSpawn" "OverrideRootScale" _asbase_character_bp 9 _asbase_character_bp 3 0.4 true 0 null null))
    (set `/Game/BluePrints/Characters/CharacterBluePrints/BaseCharacter_Bp.InventoryRef` _returnvalue _asbase_character_bp)
    (`KismetSystemLibrary.Delay` 0.5)
    (`/Game/BluePrints/Characters/CharacterBluePrints/BaseCharacter_Bp.ServerDisplayName` _asbase_character_bp)
    (bind _asgame_instance_kma (cast `/Game/BluePrints/AllLevels/GameInstance_Kma` (`GameplayStatics.GetGameInstance`)))
    (`/Game/BluePrints/AllLevels/GameInstance_Kma.ShowPlayerCount` _asgame_instance_kma)))

(event `CloseMap`
  (`Widget.RemoveFromParent` (`self.MapWidget`)))

(event `OpenMap`
  (`/Engine/EditorBlueprintResources/StandardMacros.IsValid` (`self.MapWidget`)
    (:`Is Valid`
      _)
    (:`Is Not Valid`
      (bind _returnvalue (`|CreateWidget` "/Game/UI/AllLevels/WB_MainMap.WB_MainMap_C" self))
      (set `self.MapWidget` _returnvalue)))
  (`UserWidget.AddToViewport` (`self.MapWidget`) 0))

(event `AddSpectatorScreen`
  (bind _asgame_state_kma (cast `/Game/BluePrints/AllLevels/GameState_Kma` (`GameplayStatics.GetGameState`)))
  (if (not (`/Game/BluePrints/AllLevels/GameState_Kma.GameOver?` _asgame_state_kma))
    (`WidgetLayoutLibrary.RemoveAllWidgets`)
    (bind _returnvalue (`|CreateWidget` "/Game/InventorySystem/Widgets/MainWidget.MainWidget_C" self))
    (bind _output_get (set `self.SpectatorWidget` _returnvalue))
    (`UserWidget.AddToViewport` _output_get 0)))

(event `BeginSpectating`
  (params (Killer :type "/Game/BluePrints/Characters/CharacterBluePrints/BaseCharacter_Bp Object Reference"))
  (`/Engine/EditorBlueprintResources/StandardMacros.IsValid` Killer
    (:`Is Valid`
      (set `self.KilledBy` Killer)
      (bind _returnvalue (`|SpawnActorFromClass` "/Game/BluePrints/GamePlay/Br_SpectatorPawn.Br_SpectatorPawn_C" (`self.GetTransform`) "Undefined" "OverrideRootScale" self null))
      (`self.K2_AttachToActor` _returnvalue (`self.KilledBy`) "None" "SnapToTarget" "SnapToTarget" "SnapToTarget" true)
      (`self.Possess` _returnvalue)
      (`self.AddSpectatorScreen`))
    (:`Is Not Valid`
      (`self.AddPostMatchScreen`))))

(event `AddPostMatchScreen`
  (bind _postmatchwidget (`self.PostMatchWidget`))
  (if (`self.IsLocalController`)
    (`WidgetLayoutLibrary.RemoveAllWidgets`)
    (bind _returnvalue (`|CreateWidget` "/Game/UI/AllLevels/WB_PostMatchScreen.WB_PostMatchScreen_C" self))
    (bind _output_get (set `self.PostMatchWidget` _returnvalue))
    (`UserWidget.AddToViewport` _output_get 0)
    (`WidgetBlueprintLibrary.SetInputMode_UIOnlyEx` self _postmatchwidget)
    (`UserWidget.PlayAnimation` _postmatchwidget (`/Game/UI/AllLevels/WB_PostMatchScreen.GameOver` _returnvalue) 0.0 10 "PingPong" 1.5)
    (`GameplayStatics.PlaySound2D` "/Game/Sound/Intro_Cue.Intro_Cue" 1.0 1.0 20.0 null self)))

(event `OnGameBegin`
  (if (`self.IsLocalController`)
    ;[1 1 1] Comment
    (`Widget.RemoveFromParent` (`self.LobbyWidget_2`))
    (bind _asgame_instance_kma (cast `/Game/BluePrints/AllLevels/GameInstance_Kma` (`GameplayStatics.GetGameInstance`)))
    (`Widget.RemoveFromParent` (`/Game/BluePrints/AllLevels/GameInstance_Kma.LobbyTimerRef` _asgame_instance_kma))
    (`self.ShowInGameHud`)
    (bind _asgame_state_kma (cast `/Game/BluePrints/AllLevels/GameState_Kma` (`GameplayStatics.GetGameState`)))
    (`KismetSystemLibrary.Delay` (`/Game/BP_Plane/Bp_PlanePawn.Time` (`/Game/BluePrints/AllLevels/GameState_Kma.PlanePawnRef` _asgame_state_kma)))
    (if (`self.IsOnPlane?`)
      (`self.DropFromPlane`)
      (`/Game/BluePrints/Characters/CharacterBluePrints/BaseCharacter_Bp.TellServerStartFly` (`self.CharacterRef`)))))

(event `self.ReceiveTick`
  (params (DeltaSeconds :type "Float (single-precision)")))

(event `SetFlying`)

(event `TraceDistance befor Spawn Parachute`
  (bind _asbase_character_bp (cast `/Game/BluePrints/Characters/CharacterBluePrints/BaseCharacter_Bp` (`GameplayStatics.GetPlayerPawn` 0)))
  (bind _asgame_mode_kma (cast `/Game/BluePrints/GamePlay/GameModeKma` (`GameplayStatics.GetGameMode`)))
  (for _array_element (`/Game/BluePrints/GamePlay/GameModeKma.ALivePlayersList` _asgame_mode_kma)
    (if (and (not (`/Game/BluePrints/GamePlay/PlayerControllerKma.IsOnPlane?` _array_element)) (`/Game/BluePrints/Characters/CharacterBluePrints/BaseCharacter_Bp.Flaying` _asbase_character_bp))
      (bind _camerazoom (`/Game/BluePrints/Characters/CharacterBluePrints/BaseCharacter_Bp.CameraZoom` _asbase_character_bp))
      (bind _returnvalue (`SceneComponent.K2_GetComponentLocation` _camerazoom))
      (bind (_outhit _returnvalue_2) (`KismetSystemLibrary.LineTraceSingle` _returnvalue (+ _returnvalue (* (`SceneComponent.GetForwardVector` _camerazoom) 10000.0)) "TraceTypeQuery1" false (`|MakeArray` _asbase_character_bp :!type "Actor Object Reference")))
      (if _returnvalue_2
        (set `/Game/BluePrints/Characters/CharacterBluePrints/BaseCharacter_Bp.Flaying` false _asbase_character_bp)
        (`KismetSystemLibrary.Delay` 0.1)
        (`/Game/BluePrints/Characters/CharacterBluePrints/BaseCharacter_Bp.SpawnParachute` _asbase_character_bp)
        (`GameplayStatics.PlaySound2D` "/Game/BluePrints/GamePlay/Parachute/Sound_parachute_Cue.Sound_parachute_Cue" 1.0 1.0 0.0 null null)))))

(event `ServerTraceParachute`
  (`self.TraceDistance befor Spawn Parachute`))

(event `DropFromPlane`
  (bind _returnvalue (`self.K2_GetPawn`))
  (set `self.IsOnPlane?` false)
  (bind _asgame_state_kma (cast `/Game/BluePrints/AllLevels/GameState_Kma` (`GameplayStatics.GetGameState`)))
  (bind _planepawnref (`/Game/BluePrints/AllLevels/GameState_Kma.PlanePawnRef` _asgame_state_kma))
  (`/Engine/EditorBlueprintResources/StandardMacros.IsValid` _planepawnref
    (:`Is Valid`
      (bind _returnvalue_2 (`self.GetTransform` _planepawnref))
      (`self.K2_SetActorTransform` _returnvalue _returnvalue_2 false false)
      (`self.SetControlRotation` (.rotation _returnvalue_2))
      (`self.SetViewTargetWithBlend` _returnvalue 0.5)
      (bind _asbase_character_bp (cast `/Game/BluePrints/Characters/CharacterBluePrints/BaseCharacter_Bp` (`self.K2_GetPawn`)))
      (`/Game/BluePrints/Characters/CharacterBluePrints/BaseCharacter_Bp.SetFlying` _asbase_character_bp true))))

(event `ActivateFlySound`
  (bind _asbase_character_bp (cast `/Game/BluePrints/Characters/CharacterBluePrints/BaseCharacter_Bp` (`GameplayStatics.GetPlayerPawn` 0)))
  (`ActorComponent.Activate` (`/Game/BluePrints/Characters/CharacterBluePrints/BaseCharacter_Bp.WindSound_Cue` _asbase_character_bp) false))

(event `self.ReceiveBeginPlay`
  (if (`self.IsLocalController`)
    (bind _asbase_character_bp (cast `/Game/BluePrints/Characters/CharacterBluePrints/BaseCharacter_Bp` (`GameplayStatics.GetPlayerCharacter` 0)))
    (set `self.CharacterRef` _asbase_character_bp)
    (`self.ActivateTouchInterface` "/Game/Touch/Touch_Kma.Touch_Kma")
    (`GameplayStatics.PlaySound2D` "/Game/Sound/LobbySTR_WV.LobbySTR_WV" 1.5 1.0 0.0 null self)
    (set `self.bShowMouseCursor` true)
    (bind _asgame_instance_kma (cast `/Game/BluePrints/AllLevels/GameInstance_Kma` (`GameplayStatics.GetGameInstance`)))
    (`/Game/BluePrints/AllLevels/GameInstance_Kma.ShowPlayerCount` _asgame_instance_kma)
    (`/Game/BluePrints/AllLevels/GameInstance_Kma.ShowCountDownTimer` _asgame_instance_kma)
    (bind _returnvalue (`|CreateWidget` "/Game/UI/Lobby/LobbyMenu_2.LobbyMenu_2_C" self (`self.InventoryRef`) 4))
    (bind _output_get (set `self.LobbyWidget_2` _returnvalue))
    (`UserWidget.AddToViewport` _output_get 1)))

(fn `UserConstructionScript`)