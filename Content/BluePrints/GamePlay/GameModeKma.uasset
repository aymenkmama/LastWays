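; Battle royale game mode that runs the match from player login through plane start to winner.
; BeginPlay replaces placed BaseCharacter_Bp actors with a pawn chosen from GameInstance character data, possessed by player 0.
; Pre-start logins fill player and alive lists; game start switches players' views to the plane pawn.
; Deaths on the server assign placings and update GameState's alive count, declaring the last survivor winner and triggering game over.
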(event `self.ReceiveBeginPlay`
  (`/Engine/EditorBlueprintResources/ActorMacros.Switch Has Authority`
    (:`Authority`
      (bind _asgame_instance_kma (cast `/Game/BluePrints/AllLevels/GameInstance_Kma` (`GameplayStatics.GetGameInstance`)))
      (bind _pawn (`/Game/BluePrints/AllLevels/GameInstance_Kma.CharacterData` _asgame_instance_kma))
      (`self.SpawnActor` _pawn))))

(event `self.K2_PostLogin`
  (params (NewPlayer :type "PlayerController Object Reference"))
  (bind _aliveplayerslist (`self.ALivePlayersList`))
  (bind _asgame_state_kma (cast `/Game/BluePrints/AllLevels/GameState_Kma` (`GameplayStatics.GetGameState`)))
  (if (not (`/Game/BluePrints/AllLevels/GameState_Kma.GameStarted?` _asgame_state_kma))
    (bind _asplayer_controller_kma (cast `/Game/BluePrints/GamePlay/PlayerControllerKma` NewPlayer))
    (`KismetArrayLibrary.Array_Add` (`self.PlayerList`) _asplayer_controller_kma)
    (`KismetArrayLibrary.Array_Add` _aliveplayerslist _asplayer_controller_kma)
    (set `/Game/BluePrints/AllLevels/GameState_Kma.PlayerLeftAlive` (`KismetArrayLibrary.Array_Length` _aliveplayerslist) _asgame_state_kma)))

(event `OnGameStarted`
  (`/Engine/EditorBlueprintResources/ActorMacros.Switch Has Authority`
    (:`Authority`
      (for _array_element (`self.PlayerList`)
        (set `/Game/BluePrints/GamePlay/PlayerControllerKma.IsOnPlane?` true _array_element)
        (bind _asgame_state_kma (cast `/Game/BluePrints/AllLevels/GameState_Kma` (`GameplayStatics.GetGameState`)))
        (`PlayerController.SetViewTargetWithBlend` _array_element (`/Game/BluePrints/AllLevels/GameState_Kma.PlanePawnRef` _asgame_state_kma) 0.2 "VTBlend_EaseInOut" 1.0 false)
        (`/Game/BluePrints/GamePlay/PlayerControllerKma.OnGameBegin` _array_element)))))

(event `CameraPlaneViewLeft`
  (bind _asgame_state_kma (cast `/Game/BluePrints/AllLevels/GameState_Kma` (`GameplayStatics.GetGameState`))))

(event `PlayerDied`
  (params (PlayerController :type "/Game/BluePrints/GamePlay/PlayerControllerKma Object Reference"))
  (bind _aliveplayerslist (`self.ALivePlayersList`))
  (bind _aliveplayerslist_2 (`self.ALivePlayersList`))
  (bind _returnvalue (`KismetArrayLibrary.Array_Length` _aliveplayerslist))
  ;[1 0.6983 0.6282 1 30] the last Player can't died with zone because he is the winner
  (`/Engine/EditorBlueprintResources/ActorMacros.Switch Has Authority`
    (:`Authority`
      (bind _asmy_player_state (cast `/Game/BluePrints/AllLevels/MyPlayerState` (`Controller.PlayerState` PlayerController)))
      (set `/Game/BluePrints/AllLevels/MyPlayerState.Placing` _returnvalue _asmy_player_state)
      (`KismetArrayLibrary.Array_RemoveItem` _aliveplayerslist_2 PlayerController)
      (bind _asgame_state_kma (cast `/Game/BluePrints/AllLevels/GameState_Kma` (`GameplayStatics.GetGameState`)))
      (set `/Game/BluePrints/AllLevels/GameState_Kma.PlayerLeftAlive` (`KismetArrayLibrary.Array_Length` _aliveplayerslist_2) _asgame_state_kma)
      (if (<= _returnvalue 1)
        (bind _asmy_player_state_2 (cast `/Game/BluePrints/AllLevels/MyPlayerState` (`Controller.PlayerState` (`|GetArrayItem` (`self.ALivePlayersList`) (`KismetArrayLibrary.Array_LastIndex` _aliveplayerslist)))))
        (`self.WinnerFound` _asmy_player_state_2)))))

(event `WinnerFound`
  (params (Winner :type "/Game/BluePrints/AllLevels/MyPlayerState Object Reference"))
  (set `/Game/BluePrints/AllLevels/MyPlayerState.Placing` 1 Winner)
  (bind _asgame_state_kma (cast `/Game/BluePrints/AllLevels/GameState_Kma` (`GameplayStatics.GetGameState`)))
  (`/Game/BluePrints/AllLevels/GameState_Kma.OngameOver` _asgame_state_kma))

(fn `SpawnActor`
  (params (Pawn :type String))
  (if (`KismetStringLibrary.EqualEqual_StrStr` Pawn "MalePawn")
    (bind _outactors (`GameplayStatics.GetAllActorsOfClass` "/Game/BluePrints/Characters/CharacterBluePrints/BaseCharacter_Bp.BaseCharacter_Bp_C"))
    (for _array_element _outactors
      (bind _returnvalue (`|SpawnActorFromClass` :`Class` "/Game/BluePrints/Characters/CharacterBluePrints/MainMenuPawn.MainMenuPawn_C" :`SpawnTransform` (`self.GetTransform` _array_element) :`CollisionHandlingOverride` "AlwaysSpawn" :`TransformScaleMethod` "OverrideRootScale" :`Car` null :`Instigator` null))
      (`Controller.Possess` (`GameplayStatics.GetPlayerController` 0) _returnvalue)
      (`self.K2_DestroyActor` _array_element))
    (elif (`KismetStringLibrary.EqualEqual_StrStr` Pawn "FemalePawn")
      (bind _outactors_2 (`GameplayStatics.GetAllActorsOfClass` "/Game/BluePrints/Characters/CharacterBluePrints/BaseCharacter_Bp.BaseCharacter_Bp_C"))
      (for _array_element_2 _outactors_2
        (bind _returnvalue_2 (`|SpawnActorFromClass` :`Class` "/Game/BluePrints/Characters/CharacterBluePrints/FemalePawn.FemalePawn_C" :`SpawnTransform` (`self.GetTransform` _array_element_2) :`CollisionHandlingOverride` "AlwaysSpawn" :`TransformScaleMethod` "OverrideRootScale" :`Car` null :`Instigator` null))
        (`Controller.Possess` (`GameplayStatics.GetPlayerController` 0) _returnvalue_2)
        (`self.K2_DestroyActor` _array_element_2)))))

(fn `UserConstructionScript`)