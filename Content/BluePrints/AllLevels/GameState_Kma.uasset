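; Game state that runs the lobby countdown and match start/end flow for a plane-drop, safe-zone match.
; On authority, a looping GetTimer counts down with two or more players, otherwise resets, updating TimerText-tagged text actors.
; Near zero it spawns plane pawns owned by GameMode's PlayerList entries, then BeginGame notifies the GameMode and initializes the SafeZone.
; GameOver's RepNotify shows the local player's post-match screen.
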(event `self.ReceiveBeginPlay`
  (`/Engine/EditorBlueprintResources/ActorMacros.Switch Has Authority`
    (:`Authority`
      (set `self.LobbyStarted` true)
      (`self.StartTimer`))))

(event `StartTimer`
  (bind _returnvalue (`KismetSystemLibrary.K2_SetTimer` null "GetTimer" (`self.Time`) true))
  (set `self.LobbyTimerHandle` _returnvalue))

(event `TickLobbyTimer`
  (bind _result (`/Engine/EditorBlueprintResources/StandardMacros.DecrementInt` (`self.LobbyTimer`))
    (:`  `
      (if (== _result 3)
        (`self.SpawnPlane`)
        (elif (<= _result 0)
          _)))))

(event `SpawnPlane`
  (bind _planepawnref (`self.PlanePawnRef`))
  ;[1 1 1] SpawnPlane
  (bind _asgame_mode_kma (cast `/Game/BluePrints/GamePlay/GameModeKma` (`GameplayStatics.GetGameMode`)))
  (for _array_element (`/Game/BluePrints/GamePlay/GameModeKma.PlayerList` _asgame_mode_kma)
    (if (== _array_element _array_element)
      (bind _returnvalue (`|SpawnActorFromClass` "/Game/BP_Plane/Bp_PlanePawn.Bp_PlanePawn_C" (`self.GetTransform`) "AlwaysSpawn" "OverrideRootScale" _array_element null))
      (set `self.PlanePawnRef` _returnvalue)
      (if (== (`self.GetLifeSpan` _planepawnref) 130.0)
        (`self.K2_DestroyActor` _planepawnref)))))

(event `BeginGame`
  (bind _safezone (`self.SafeZone`))
  (`KismetSystemLibrary.K2_ClearAndInvalidateTimerHandle` (`self.LobbyTimerHandle`))
  (set `self.GameStarted?` true)
  (bind _asgame_mode_kma (cast `/Game/BluePrints/GamePlay/GameModeKma` (`GameplayStatics.GetGameMode`)))
  (`/Game/BluePrints/GamePlay/GameModeKma.OnGameStarted` _asgame_mode_kma)
  (`/Engine/EditorBlueprintResources/StandardMacros.IsValid` _safezone
    (:`Is Valid`
      (`/Game/BluePrints/Zone/CircleZone_Bp.InitZone` _safezone))))

(event `OngameOver`
  (set `self.GameOver?` true))

(event `ClientSpawnPlane`
  (params (SpawnTransform :type "Transform Structure") (PlayerController :type "/Game/BluePrints/GamePlay/PlayerControllerKma Object Reference") (PlanePawnRef :type "/Game/BP_Plane/Bp_PlanePawn Object Reference"))
  (bind _returnvalue (`|SpawnActorFromClass` "/Game/BP_Plane/Bp_PlanePawn.Bp_PlanePawn_C" SpawnTransform "AlwaysSpawn" "OverrideRootScale" PlayerController PlanePawnRef))
  (set `self.PlanePawnRef` _returnvalue))

(event `ServerSpawnPlane`
  (params (SpawnTransform :type "Transform Structure") (PlayerController :type "/Game/BluePrints/GamePlay/PlayerControllerKma Object Reference") (PlanePawnRef :type "/Game/BP_Plane/Bp_PlanePawn Object Reference"))
  (`self.ClientSpawnPlane` SpawnTransform PlayerController PlanePawnRef))

(fn `GetTimer`
  (if (>= (`self.PlayerLeftAlive`) 2)
    (set `self.LobbyStarted` true)
    (bind _result (`/Engine/EditorBlueprintResources/StandardMacros.DecrementInt` (`self.Seconds`))
      (:`  `
        (if (== (`self.Seconds`) 3)
          (`self.SpawnPlane`))
        (set `self.Seconds` _result)
        (if (< (`self.Seconds`) 0)
          (bind _result_2 (`/Engine/EditorBlueprintResources/StandardMacros.DecrementInt` (`self.Mins`))
            (:`  `
              (set `self.Mins` _result_2)
              (set `self.Seconds` 59)
              (`self.SetText` (`self.Mins`) (`self.Seconds`))))
          (else
            (`self.SetText` (`self.Mins`) (`self.Seconds`))))
        (if (and (<= (`self.Seconds`) 0) (<= (`self.Mins`) 0))
          (`self.BeginGame`)
          (set `self.LobbyStarted` false))))
    (else
      ;[1 1 1] Pause and Reset the Timer
      (set `self.Time` (- (`self.Time`) 2.0))
      (set `self.Mins` 0)
      (set `self.Seconds` 5))))

(fn `OnRep_GameOver?`
  (if (`self.GameOver?`)
    (bind _asplayer_controller_kma (cast `/Game/BluePrints/GamePlay/PlayerControllerKma` (`GameplayStatics.GetPlayerController` 0)))
    (`/Game/BluePrints/GamePlay/PlayerControllerKma.AddPostMatchScreen` _asplayer_controller_kma)))

(fn `SetText`
  (params (Mins :type Integer) (Seconds :type Integer))
  (bind _outactors (`GameplayStatics.GetAllActorsWithTag` "TimerText"))
  (for _array_element _outactors
    (`TextRenderComponent.K2_SetText` (`self.GetComponentByClass` _array_element "/Script/Engine.TextRenderComponent") (`|FormatText` "{Mins}:{Seconds}" Mins Seconds))))

(fn `UserConstructionScript`)