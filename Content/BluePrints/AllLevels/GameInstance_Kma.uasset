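; Game instance that handles online session matchmaking, shared UI screens and the saved character choice.
; TryJoinOrCreateSession clears any existing session, then joins the first one found or hosts GamePlayMap as a listen server; CreateSession hosts directly.
; Loading, lobby countdown and player count widgets are created once and cached, the latter two gated by GameState_Kma flags; ShowMainMenue is empty.
; CharacterData returns the pawn saved in MainMenuCharacter, defaulting to MalePawn.
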(event `ShowMainMenue`)

(event `ShowPlayerCount`
  (bind _asgame_state_kma (cast `/Game/BluePrints/AllLevels/GameState_Kma` (`GameplayStatics.GetGameState`)))
  (if (`/Game/BluePrints/AllLevels/GameState_Kma.GameStarted?` _asgame_state_kma)
    (`/Engine/EditorBlueprintResources/StandardMacros.IsValid` (`self.ConnectedPlayersRef`)
      (:`Is Valid`
        _)
      (:`Is Not Valid`
        (bind _returnvalue (`|CreateWidget` "/Game/UI/AllLevels/ConnectedPlayers.ConnectedPlayers_C" (`GameplayStatics.GetPlayerController` 0)))
        (set `self.ConnectedPlayersRef` _returnvalue)))
    (`UserWidget.AddToViewport` (`self.ConnectedPlayersRef`) 0)))

(event `self.ReceiveInit`
  (set `self.MainMenueRef` (`self.MainMenueRef`))
  (set `self.LoandingScreenRef` (`self.LoandingScreenRef`))
  (set `self.LobbyTimerRef` (`self.LobbyTimerRef`))
  (set `self.ConnectedPlayersRef` (`self.ConnectedPlayersRef`)))

(event `ShowLoading Screen`
  (`/Engine/EditorBlueprintResources/StandardMacros.IsValid` (`self.LoandingScreenRef`)
    (:`Is Valid`
      _)
    (:`Is Not Valid`
      (bind _returnvalue (`|CreateWidget` "/Game/UI/AllLevels/LoadingScreen.LoadingScreen_C" (`GameplayStatics.GetPlayerController` 0)))
      (set `self.LoandingScreenRef` _returnvalue)))
  (`UserWidget.AddToViewport` (`self.LoandingScreenRef`) 0))

(event `ShowCountDownTimer`
  (bind _asgame_state_kma (cast `/Game/BluePrints/AllLevels/GameState_Kma` (`GameplayStatics.GetGameState`)))
  (if (and (`/Game/BluePrints/AllLevels/GameState_Kma.LobbyStarted` _asgame_state_kma) (not (`/Game/BluePrints/AllLevels/GameState_Kma.GameStarted?` _asgame_state_kma)))
    (`/Engine/EditorBlueprintResources/StandardMacros.IsValid` (`self.LobbyTimerRef`)
      (:`Is Valid`
        _)
      (:`Is Not Valid`
        (bind _returnvalue (`|CreateWidget` "/Game/UI/Lobby/LobbyTimer.LobbyTimer_C" (`GameplayStatics.GetPlayerController` 0)))
        (set `self.LobbyTimerRef` _returnvalue)))
    (`UserWidget.AddToViewport` (`self.LobbyTimerRef`) 0)))

(event `CreateSession`
  (`self.ShowLoading Screen`)
  (`CreateSessionCallbackProxy.CreateSession` (`GameplayStatics.GetPlayerController` 0) 60
    (:`OnSuccess`
      (`GameplayStatics.OpenLevel` "GamePlayMap" true "listen"))))

(event `TryJoinOrCreateSession`
  (bind _returnvalue (`GameplayStatics.GetPlayerController` 0))
  (`DestroySessionCallbackProxy.DestroySession` _returnvalue
    (:`OnSuccess`
      _)
    (:`OnFailure`
      _))
  (`self.ShowLoading Screen`)
  (bind _results (`FindSessionsCallbackProxy.FindSessions` _returnvalue 20)
    (:`OnSuccess`
      (if (`KismetArrayLibrary.Array_IsValidIndex` _results)
        (`self.JoinBPSession` (`|GetArrayItem` _results))
        (else
          (`CreateSessionCallbackProxy.CreateSession` (`GameplayStatics.GetPlayerController` 0) 50 :!label _label
            (:`then`
              (`GameplayStatics.OpenLevel` "GamePlayMap" true "listen"))
            (:`OnFailure`
              (`KismetSystemLibrary.PrintString` "Error To Create Session" true true (struct :`R` 1.0 :`G` 0.401258 :`A` 1.0) 5.0))))))
    (:`OnFailure`
      (goto _label))))

(event `JoinBPSession`
  (params (Session :type "BlueprintSessionResult Structure"))
  (`JoinSessionCallbackProxy.JoinSession` (`GameplayStatics.GetPlayerController` 0) Session
    (:`OnFailure`
      (`KismetSystemLibrary.PrintString` "Failed To Join Session" true true (struct :`G` 0.294829 :`B` 1.0 :`A` 1.0) 5.0))))

(fn `CharacterData`
  (returns (Pawn :type String))
  (bind _returnvalue (`GameplayStatics.DoesSaveGameExist` "MainMenuCharacter"))
  (if _returnvalue
    (bind _returnvalue_2 (`GameplayStatics.LoadGameFromSlot` "MainMenuCharacter"))
    (bind _assave_main_menu_player (cast `/Game/BluePrints/AllLevels/SaveMainMenuPlayer` _returnvalue_2)
      (:`then`
        (return (`/Game/BluePrints/AllLevels/SaveMainMenuPlayer.Pawn` _assave_main_menu_player)))
      (:`CastFailed`
        (return "MalePawn")))
    (else
      (`KismetSystemLibrary.PrintString` "NoSaveGame")
      (return "MalePawn"))))