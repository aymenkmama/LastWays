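; Zipline actor that carries a player along a spline, with a cable and capsule fitted to the spline in the construction script.
; Interaction routes through server and multicast-named events to Zipping, which starts the ride or ends one already playing.
; A timeline seeded from the player's distance along the line moves them below it, with an attached handle actor and sound.
; Rides only start facing along the arrow; the reverse branch is unwired.
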(event `self.ReceiveBeginPlay`
  (`TimelineComponent.SetPlayRate` (`self.ZipTimeline`) (`self.PlayRate`)))

(event `Zipping`
  (params (Player :type "/Game/BluePrints/Characters/CharacterBluePrints/BaseCharacter_Bp Object Reference"))
  (bind _zipline (`self.ZipLine`))
  (bind _zipline_2 (`self.ZipLine`))
  (bind _ziplinesound (`/Game/BluePrints/Characters/CharacterBluePrints/BaseCharacter_Bp.ZipLineSound` Player))
  (bind _spline (`self.Spline`))
  (set `self.PlayerRef` Player)
  (if (`TimelineComponent.IsPlaying` (`self.ZipTimeline`))
    (set `self.FinishZip` true)
    (`/Engine/EditorBlueprintResources/StandardMacros.IsValid` Player
      (:`Is Valid`
        (`/Game/BluePrints/Characters/CharacterBluePrints/BaseCharacter_Bp.ServerZiplineStop` Player)
        (`/Engine/EditorBlueprintResources/StandardMacros.IsValid` _zipline_2
          (:`Is Valid`
            (`self.K2_DestroyActor` _zipline_2)
            (`ActorComponent.Deactivate` _ziplinesound)
            (bind (_direction _traveldistance) (`Timeline|ZipTimeline` :!via `Stop` :!label _label)
              (:`Update`
                (`/Engine/EditorBlueprintResources/StandardMacros.IsValid` Player
                  (:`Is Valid`
                    (bind (_returnvalue_x _returnvalue_y _returnvalue_z) (`KismetMathLibrary.BreakVector` (`SplineComponent.GetLocationAtDistanceAlongSpline` _spline (* _traveldistance (`SplineComponent.GetSplineLength` _spline)) "World")))
                    (`self.K2_SetActorLocation` Player (`KismetMathLibrary.MakeVector` _returnvalue_x _returnvalue_y (- _returnvalue_z 135.0)) false false)
                    (set `self.FinishZip` true))))
              (:`Finished`
                (set `self.FinishZip` true)
                (`/Engine/EditorBlueprintResources/StandardMacros.IsValid` Player
                  (:`Is Valid`
                    (`/Game/BluePrints/Characters/CharacterBluePrints/BaseCharacter_Bp.ServerZiplineStop` Player)
                    (`/Engine/EditorBlueprintResources/StandardMacros.IsValid` _zipline
                      (:`Is Valid`
                        (`self.K2_DestroyActor` _zipline)
                        (`ActorComponent.Deactivate` _ziplinesound)))))))))))
    (else
      (`self.GetDistanceRatio` Player)
      (bind _direction_2 (`self.DitectDirection` Player))
      (bind _output_get (set `self.Direction` _direction_2))
      (if (>= _output_get 0.0)
        (`/Engine/EditorBlueprintResources/StandardMacros.IsValid` Player
          (:`Is Valid`
            (`/Game/BluePrints/Characters/CharacterBluePrints/BaseCharacter_Bp.ServerZiplineStart` Player)
            (`self.SpawnZip` Player)
            (`ActorComponent.Activate` _ziplinesound false)
            (goto _label)))))))

(event `MultiZipping`
  (params (Object :type "/Game/BluePrints/Characters/CharacterBluePrints/BaseCharacter_Bp Object Reference"))
  (`self.Zipping` Object))

(event `Zip`
  (params (Object :type "/Game/BluePrints/Characters/CharacterBluePrints/BaseCharacter_Bp Object Reference"))
  (`self.MultiZipping` Object))

(event `/Game/BluePrints/Zipline/BPI_ZipLineIneraction.Interaction`
  (params (Player :type "/Game/BluePrints/Characters/CharacterBluePrints/BaseCharacter_Bp Object Reference"))
  (`/Engine/EditorBlueprintResources/ActorMacros.Switch Has Authority`
    (:`Authority`
      (`self.Zip` Player))
    (:`Remote`
      (`self.ServerZipping` Player))))

(event `ServerZipping`
  (params (Object :type "/Game/BluePrints/Characters/CharacterBluePrints/BaseCharacter_Bp Object Reference"))
  (`self.Zip` Object))

(fn `CapsuleCollision`
  (locals (LocalHalfLenght :type "Float (double-precision)" :default 0.0))
  (bind _localhalflenght (`local.LocalHalfLenght`))
  (bind _returnvalue (`SplineComponent.GetTransformAtDistanceAlongSpline` (`self.Spline`) _localhalflenght "World" false))
  (set `local.LocalHalfLenght` (/ (`SplineComponent.GetSplineLength` (`self.Spline`)) 2.0))
  (`CapsuleComponent.SetCapsuleHalfHeight` (`self.Capsule`) _localhalflenght true)
  (`SceneComponent.K2_SetWorldTransform` (`self.Capsule`) (`KismetMathLibrary.MakeTransform` (.location _returnvalue) (`KismetMathLibrary.MakeRotator` (.roll (.rotation _returnvalue)) (+ (.pitch (.rotation _returnvalue)) 90.0) (.yaw (.rotation _returnvalue)))) false false))

(fn `ConstructCable`
  (bind _cable (`self.Cable`))
  (bind _cable_2 (`self.Cable`))
  (`SceneComponent.K2_SetWorldLocation` _cable (`SplineComponent.GetLocationAtSplinePoint` (`self.Spline`) 0 "World") false false)
  (set `CableComponent.bAttachEnd` true _cable_2)
  (set `CableComponent.EndLocation` (`SplineComponent.GetLocationAtSplinePoint` (`self.Spline`) 1 "Local") _cable_2)
  (set `CableComponent.CableLength` (`SplineComponent.GetSplineLength` (`self.Spline`)) (`self.Cable`))
  (`PrimitiveComponent.SetEnableGravity` _cable false))

(fn `DitectDirection`
  (params (Player :type "/Game/BluePrints/Characters/CharacterBluePrints/BaseCharacter_Bp Object Reference"))
  (returns (Direction :type "Float (double-precision)"))
  (`/Engine/EditorBlueprintResources/StandardMacros.IsValid` Player
    (:`Is Valid`
      (return (`KismetMathLibrary.Dot_VectorVector` (`KismetMathLibrary.GetForwardVector` (`SceneComponent.K2_GetComponentRotation` (`Character.Mesh` Player))) (`KismetMathLibrary.GetForwardVector` (`SceneComponent.K2_GetComponentRotation` (`self.Arrow`))))))))

(fn `GetDistanceRatio`
  (params (Player :type "/Game/BluePrints/Characters/CharacterBluePrints/BaseCharacter_Bp Object Reference"))
  (bind _ziptimeline (`self.ZipTimeline`))
  (`/Engine/EditorBlueprintResources/StandardMacros.IsValid` Player
    (:`Is Valid`
      (`TimelineComponent.SetNewTime` _ziptimeline (* (`TimelineComponent.GetTimelineLength` _ziptimeline) (/ (`KismetMathLibrary.VSize` (- (`self.K2_GetActorLocation` Player) (`SplineComponent.GetLocationAtSplinePoint` (`self.Spline`) 0 "World"))) (`SplineComponent.GetSplineLength` (`self.Spline`))))))))

(fn `SpawnZip`
  (params (Player :type "Character Object Reference"))
  (returns (ReturnValue :type Boolean))
  (bind _returnvalue (`|SpawnActorFromClass` "/Game/Geometry/ZipLine/Bp_BldZipLow.Bp_BldZipLow_C" (`KismetMathLibrary.MakeTransform` (0.0 0.0 0.0)) "AlwaysSpawn" "OverrideRootScale" null null))
  (bind _output_get (set `self.ZipLine` _returnvalue))
  (bind _returnvalue_2 (`SceneComponent.K2_AttachToComponent` (`/Game/Geometry/ZipLine/Bp_BldZipLow.StaticMesh` _output_get) (`Character.Mesh` Player) "ZipLine" "SnapToTarget" "SnapToTarget" "SnapToTarget" true))
  (if _returnvalue_2
    (return _returnvalue_2)
    (else
      (return false))))

(fn `UserConstructionScript`
  (`self.ConstructCable` self)
  (`self.CapsuleCollision` self))