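; Plane pawn that flies across the map at fixed height and speed, viewed through a spring-arm camera.
; On BeginPlay, the authority sets up input and camera, derives opposite-side endpoints with random yaw variation, and sets lifespan from flight time.
; Start direction feeds random degree values into arccosine and arcsine, outside their valid input range.
; Tick moves it toward the endpoint and spins four turbines at a frame-rate-dependent rate.
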(event `self.ReceiveBeginPlay`
  (bind _springarm (`self.SpringArm`))
  (`/Engine/EditorBlueprintResources/ActorMacros.Switch Has Authority`
    (:`Authority`
      (`self.EnableInput` (`GameplayStatics.GetPlayerController` 0))
      (set `SpringArmComponent.TargetArmLength` 3000.0 _springarm)
      (set `SpringArmComponent.TargetOffset` (0.0 0.0 100.0) _springarm)
      (bind _output_get (set `self.Time` (/ (`self.MapSize`) (`self.FlySpeed`))))
      (`self.SetLifeSpan` (+ _output_get 10.0))
      (bind _output_get_2 (set `self.CenterOffset` (`KismetMathLibrary.Normal` (`KismetMathLibrary.MakeVector` (`KismetMathLibrary.DegAcos` (`KismetMathLibrary.RandomFloatInRange` -180.0 180.0)) (`KismetMathLibrary.DegAsin` (`KismetMathLibrary.RandomFloatInRange` -180.0 180.0))))))
      (set `self.FlightPathStart` (* _output_get_2 (/ (`self.MapSize`) 2.0)))
      (set `self.FlightPathEnd` (* (`KismetMathLibrary.GreaterGreater_VectorRotator` (* (`self.CenterOffset`) -1.0) (`KismetMathLibrary.MakeRotator` 0.0 0.0 (`KismetMathLibrary.RandomFloatInRange` -15.0 15.0))) (/ (`self.MapSize`) 2.0)))
      (`self.K2_SetActorRotation` (`KismetMathLibrary.Conv_VectorToRotator` (- (`self.FlightPathEnd`) (`self.FlightPathStart`))))
      (`self.K2_SetActorLocation` (`self.FlightPathStart`))
      (`SceneComponent.K2_SetRelativeRotation` (`self.SpringArm`) (`SceneComponent.RelativeRotation` (`self.PlaneCamera`)) false false))))

(event `self.ReceiveTick`
  (params (DeltaSeconds :type "Float (single-precision)"))
  (`self.K2_SetActorLocation` (`KismetMathLibrary.MakeVector` (.x (`KismetMathLibrary.VInterpTo_Constant` (`self.K2_GetActorLocation`) (`self.FlightPathEnd`) DeltaSeconds (`self.FlySpeed`))) (.y (`KismetMathLibrary.VInterpTo_Constant` (`self.K2_GetActorLocation`) (`self.FlightPathEnd`) DeltaSeconds (`self.FlySpeed`))) (`self.FlyHeight`)))
  (`SceneComponent.K2_AddLocalRotation` (`self.Turbine_1`) (struct :`Roll` 30.0) false false)
  (`SceneComponent.K2_AddLocalRotation` (`self.Turbine_2`) (struct :`Roll` 30.0) false false)
  (`SceneComponent.K2_AddLocalRotation` (`self.Turbine_3`) (struct :`Roll` 30.0) false false)
  (`SceneComponent.K2_AddLocalRotation` (`self.Turbine_4`) (struct :`Roll` 30.0) false false))

(fn `OnRep_FrontCamera`)

(fn `UserConstructionScript`)