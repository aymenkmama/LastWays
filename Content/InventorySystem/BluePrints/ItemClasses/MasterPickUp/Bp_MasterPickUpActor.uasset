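; Base world pickup actor that offers an item class and amount for characters to add to their inventory.
; Sphere overlaps maintain each character's NearByPickUpActors queue, showing the name, amount and icon widget for the first entry and promoting the next.
; Overlaps update locally controlled characters directly and also call Server-named events on remote instances.
; PickUp adds to inventory, then zeroes Amount if a remainder returns, otherwise dequeues and destroys itself.
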(event `ShowingPickUpWidget`
  (params (Player :type "/Game/BluePrints/Characters/CharacterBluePrints/BaseCharacter_Bp Object Reference"))
  (bind _asbase_character_bp (cast `/Game/BluePrints/Characters/CharacterBluePrints/BaseCharacter_Bp` Player))
  (bind _inventoryref (`/Game/BluePrints/Characters/CharacterBluePrints/BaseCharacter_Bp.InventoryRef` _asbase_character_bp))
  (`/Engine/EditorBlueprintResources/StandardMacros.IsValid` _inventoryref
    (:`Is Valid`
      (bind _nearbypickupactors (`/Game/BluePrints/Characters/CharacterBluePrints/BaseCharacter_Bp.NearByPickUpActors` _asbase_character_bp))
      (if (> (`KismetArrayLibrary.Array_Length` _nearbypickupactors) 0)
        (`KismetArrayLibrary.Array_Add` _nearbypickupactors self)
        (else
          (`SceneComponent.SetVisibility` (`self.PickUpWidget`) true false)
          (`KismetArrayLibrary.Array_Add` _nearbypickupactors self)
          (`Widget.SetVisibility` (`/Game/UI/Lobby/LobbyMenu.PickUpItem` (`/Game/InventorySystem/Bp_Inventory.LobbyWidget` _inventoryref)) "Visible"))))))

(event `self.ReceiveBeginPlay`
  (bind _asbase_character_bp (cast `/Game/BluePrints/Characters/CharacterBluePrints/BaseCharacter_Bp` (`GameplayStatics.GetPlayerCharacter` 0)))
  (set `self.Player` _asbase_character_bp)
  (`self.UpdatePickUpWidget`))

(event `DestroyActor`
  (`self.K2_DestroyActor` self))

(event `MultiDestroy`
  (`self.DestroyActor`))

(event `ServerShowingWidget`
  (params (Player :type "/Game/BluePrints/Characters/CharacterBluePrints/BaseCharacter_Bp Object Reference"))
  (`self.ShowingPickUpWidget` Player))

(event `ServerDestroy`
  (`KismetSystemLibrary.Delay` 0.001)
  (`self.MultiDestroy`))

(event `self.Sphere.OnComponentBeginOverlap`
  (params (OverlappedComponent :type "PrimitiveComponent Object Reference") (OtherActor :type "Actor Object Reference") (OtherComp :type "PrimitiveComponent Object Reference") (OtherBodyIndex :type Integer) (bFromSweep :type Boolean) (SweepResult :type "HitResult Structure (by ref)"))
  (bind _asbase_character_bp (cast `/Game/BluePrints/Characters/CharacterBluePrints/BaseCharacter_Bp` OtherActor))
  (`/Engine/EditorBlueprintResources/ActorMacros.Switch Has Authority`
    (:`Authority`
      _)
    (:`Remote`
      (`self.ServerShowingWidget` _asbase_character_bp)))
  (if (`Pawn.IsLocallyControlled` _asbase_character_bp)
    (`self.ShowingPickUpWidget` _asbase_character_bp)))

(event `ServerHideWidget`
  (params (Player :type "/Game/BluePrints/Characters/CharacterBluePrints/BaseCharacter_Bp Object Reference"))
  (`self.HidePickUpWidget` Player))

(event `HidePickUpWidget`
  (params (Player :type "/Game/BluePrints/Characters/CharacterBluePrints/BaseCharacter_Bp Object Reference"))
  (bind _asbase_character_bp (cast `/Game/BluePrints/Characters/CharacterBluePrints/BaseCharacter_Bp` Player))
  (bind _nearbypickupactors (`/Game/BluePrints/Characters/CharacterBluePrints/BaseCharacter_Bp.NearByPickUpActors` _asbase_character_bp))
  (bind _output (`|GetArrayItem` _nearbypickupactors))
  (if (and (`KismetSystemLibrary.IsValid` _output) (== _output self))
    (`SceneComponent.SetVisibility` (`self.PickUpWidget`) false false)
    (bind _pickupitem (`/Game/UI/Lobby/LobbyMenu.PickUpItem` (`/Game/InventorySystem/Bp_Inventory.LobbyWidget` (`/Game/BluePrints/Characters/CharacterBluePrints/BaseCharacter_Bp.InventoryRef` _asbase_character_bp))))
    (`Widget.SetVisibility` _pickupitem "Hidden")
    (`KismetArrayLibrary.Array_RemoveItem` _nearbypickupactors self)
    (bind _output_2 (`|GetArrayItem` (`/Game/BluePrints/Characters/CharacterBluePrints/BaseCharacter_Bp.NearByPickUpActors` _asbase_character_bp)))
    (`/Engine/EditorBlueprintResources/StandardMacros.IsValid` _output_2
      (:`Is Valid`
        (`SceneComponent.SetVisibility` (`/Game/InventorySystem/BluePrints/ItemClasses/MasterPickUp/Bp_MasterPickUpActor.PickUpWidget` _output_2) true false)
        (`Widget.SetVisibility` _pickupitem "Hidden")))
    (else
      (`KismetArrayLibrary.Array_RemoveItem` _nearbypickupactors self))))

(event `self.Sphere.OnComponentEndOverlap`
  (params (OverlappedComponent :type "PrimitiveComponent Object Reference") (OtherActor :type "Actor Object Reference") (OtherComp :type "PrimitiveComponent Object Reference") (OtherBodyIndex :type Integer))
  (bind _asbase_character_bp (cast `/Game/BluePrints/Characters/CharacterBluePrints/BaseCharacter_Bp` OtherActor))
  (`/Engine/EditorBlueprintResources/ActorMacros.Switch Has Authority`
    (:`Authority`
      _)
    (:`Remote`
      (`self.ServerHideWidget` _asbase_character_bp)))
  (if (`Pawn.IsLocallyControlled` _asbase_character_bp)
    (`/Engine/EditorBlueprintResources/StandardMacros.IsValid` _asbase_character_bp
      (:`Is Valid`
        (`self.HidePickUpWidget` _asbase_character_bp)))))

(fn `PickUp`
  (params (Inventory :type "/Game/InventorySystem/Bp_Inventory Object Reference") (Character :type "/Game/BluePrints/Characters/CharacterBluePrints/BaseCharacter_Bp Object Reference") (Item :type "/Game/InventorySystem/BluePrints/ItemClasses/MasterPickUp/Bp_MasterPickUpActor Object Reference (by ref)"))
  (bind _nearbypickupactors (`/Game/BluePrints/Characters/CharacterBluePrints/BaseCharacter_Bp.NearByPickUpActors` Character))
  (bind _output (`|GetArrayItem` _nearbypickupactors))
  (`/Engine/EditorBlueprintResources/StandardMacros.IsValid` Inventory
    (:`Is Valid`
      (bind (_sucess_ _reste) (`/Game/InventorySystem/Bp_Inventory.AddItem` Inventory (`self.ItemToAdd`) (`self.Amount`) true))
      (if _sucess_
        (if (> _reste 0)
          (set `self.Amount` 0)
          (`self.UpdatePickUpWidget`)
          (return)
          (else
            (bind _returnvalue (`KismetArrayLibrary.Array_RemoveItem` _nearbypickupactors Item))
            (if _returnvalue
              (`/Engine/EditorBlueprintResources/StandardMacros.IsValid` _output
                (:`Is Valid`
                  (`SceneComponent.SetVisibility` (`/Game/InventorySystem/BluePrints/ItemClasses/MasterPickUp/Bp_MasterPickUpActor.PickUpWidget` _output) true false)
                  (`self.K2_DestroyActor` self)
                  (return))
                (:`Is Not Valid`
                  (`self.K2_DestroyActor` self)
                  (return))))))))))

(fn `UpdatePickUpWidget`
  (bind (_name _description _icon) (break `/Game/InventorySystem/BluePrints/Structures/S_iteminfo` (defaults `/Game/InventorySystem/BluePrints/ItemClasses/MasterPickUp/Bp_MasterPickUpActor` (`self.ItemToAdd`))))
  (bind _aspick_up_widget (cast `/Game/InventorySystem/Widgets/PickUpWidget` (`WidgetComponent.GetUserWidgetObject` (`self.PickUpWidget`)))
    (:`then`
      (`TextBlock.SetText` (`/Game/InventorySystem/Widgets/PickUpWidget.NameText` _aspick_up_widget) (`|FormatText` "{Name} ({Amount})" _name (`self.Amount`)))
      (`Image.SetBrushFromTexture` (`/Game/InventorySystem/Widgets/PickUpWidget.ItemIcon` _aspick_up_widget) _icon false))
    (:`CastFailed`
      _))
  (return))

(fn `UserConstructionScript`)