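; Base Blueprint for inventory items, apparently meant as the parent of specific item classes.
; On BeginPlay it caches player 0's pawn as a BaseCharacter_Bp reference, and it exposes an OnUsed event with an empty body.
; Disconnected, never-executed graphs hold use logic: authority-checked removal from the inventory, category-based server healing and actor destruction.
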(event `self.ReceiveBeginPlay`
  (bind _asbase_character_bp (cast `/Game/BluePrints/Characters/CharacterBluePrints/BaseCharacter_Bp` (`GameplayStatics.GetPlayerPawn` 0)))
  (set `self.PlayerRef` _asbase_character_bp))

(event `OnUsed`
  (params (Character :type "/Game/BluePrints/Characters/CharacterBluePrints/BaseCharacter_Bp Object Reference")))

(fn `UserConstructionScript`)