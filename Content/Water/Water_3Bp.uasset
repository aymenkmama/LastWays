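; Water volume actor that deals environmental damage over time to players not on the plane.
; Begin overlap on the water component plays a splash sound for each off-plane player in the game mode's alive list and sets a shared Overlapping flag; end overlap clears it.
; While the flag is set, Tick damages every such player's pawn, scaled by delta time, regardless of which actor overlapped.
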(event `self.ReceiveTick`
  (params (DeltaSeconds :type "Float (single-precision)"))
  (bind _asgame_mode_kma (cast `/Game/BluePrints/GamePlay/GameModeKma` (`GameplayStatics.GetGameMode`)))
  (for _array_element (`/Game/BluePrints/GamePlay/GameModeKma.ALivePlayersList` _asgame_mode_kma)
    (`/Engine/EditorBlueprintResources/StandardMacros.IsValid` _array_element
      (:`Is Valid`
        (if (and (`self.Overlapping`) (not (`/Game/BluePrints/GamePlay/PlayerControllerKma.IsOnPlane?` _array_element)))
          (`GameplayStatics.ApplyDamage` (`Controller.K2_GetPawn` _array_element) (* DeltaSeconds (`self.WaterDamage`)) null self "/Engine/EngineDamageTypes/DmgTypeBP_Environmental.DmgTypeBP_Environmental_C"))))))

(event `self.Water_2.OnComponentBeginOverlap`
  (params (OverlappedComponent :type "PrimitiveComponent Object Reference") (OtherActor :type "Actor Object Reference") (OtherComp :type "PrimitiveComponent Object Reference") (OtherBodyIndex :type Integer) (bFromSweep :type Boolean) (SweepResult :type "HitResult Structure (by ref)"))
  (bind _asgame_mode_kma (cast `/Game/BluePrints/GamePlay/GameModeKma` (`GameplayStatics.GetGameMode`)))
  (for _array_element (`/Game/BluePrints/GamePlay/GameModeKma.ALivePlayersList` _asgame_mode_kma)
    (if (not (`/Game/BluePrints/GamePlay/PlayerControllerKma.IsOnPlane?` _array_element))
      (`GameplayStatics.PlaySoundAtLocation` "/Game/Sounds/WaterSounds/WaterSplash_Cue.WaterSplash_Cue" (`.Location` (`GameplayStatics.BreakHitResult` SweepResult)) (struct) 1.0 1.0 0.0 null null (`Controller.K2_GetPawn` _array_element))
      (set `self.Overlapping` true))))

(event `self.Water_2.OnComponentEndOverlap`
  (params (OverlappedComponent :type "PrimitiveComponent Object Reference") (OtherActor :type "Actor Object Reference") (OtherComp :type "PrimitiveComponent Object Reference") (OtherBodyIndex :type Integer))
  (bind _asgame_mode_kma (cast `/Game/BluePrints/GamePlay/GameModeKma` (`GameplayStatics.GetGameMode`)))
  (for _array_element (`/Game/BluePrints/GamePlay/GameModeKma.ALivePlayersList` _asgame_mode_kma)
    (set `self.Overlapping` false)))

(fn `UserConstructionScript`)